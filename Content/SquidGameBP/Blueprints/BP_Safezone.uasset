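; BP_Safezone is a trigger zone that decides whether a BP_SquidPerson leaving it counts as safe.
; On box end overlap, it multiplies the arrow's forward X by the character's X offset from the arrow, setting IsSafe true if positive (exited forward), false otherwise, with debug prints.
; A separate SetCollisionPreset event changes the box's collision profile after a given delay.
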(event `self.Box.OnComponentEndOverlap`
  (params (OverlappedComponent :type "PrimitiveComponent Object Reference") (OtherActor :type "Actor Object Reference") (OtherComp :type "PrimitiveComponent Object Reference") (OtherBodyIndex :type Integer))
  (bind _arrow (`self.Arrow`))
  (bind _returnvalue_x (`KismetMathLibrary.BreakVector` (`SceneComponent.GetForwardVector` _arrow)))
  (bind _returnvalue_x_2 (`KismetMathLibrary.BreakVector` (`SceneComponent.K2_GetComponentLocation` _arrow)))
  (bind _asbp_squid_person (cast `/Game/SquidGameBP/Gamemode/BP_SquidPerson` OtherActor))
  (bind _returnvalue_x_3 (`KismetMathLibrary.BreakVector` (`self.K2_GetActorLocation` _asbp_squid_person)))
  (if (> (* _returnvalue_x (- _returnvalue_x_3 _returnvalue_x_2)) 0.0)
    (`KismetSystemLibrary.PrintString` "통과")
    (set `/Game/SquidGameBP/Gamemode/BP_SquidPerson.IsSafe` true _asbp_squid_person)
    (else
      (`KismetSystemLibrary.PrintString` "불통")
      (set `/Game/SquidGameBP/Gamemode/BP_SquidPerson.IsSafe` false _asbp_squid_person))))

(event `SetCollisionPreset`
  (params (delaytime :type "Float (double-precision)") (ProfileName :type Name))
  (`KismetSystemLibrary.Delay` delaytime)
  (`PrimitiveComponent.SetCollisionProfileName` (`self.Box`) ProfileName true))

(fn `UserConstructionScript`)