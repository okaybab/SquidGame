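; BP_Timer is an in-world match timer that shows MM:SS on a text render and fires OnGameTimeOut at 00:00.
; BeginPlay sets the starting seconds from the game instance's difficulty level and binds the start event to the game mode's OnLevelStartUp dispatcher.
; After a short delay, a looping function timer steps the time by Speed, clamps and zero-pads it, updating text only when the string changes.
; Reaching 00:00 also stops the timer.
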(event `self.ReceiveBeginPlay`
  (`|ExecutionSequence`
    (:`then_0`
      (bind _asbp_squid_instance (cast `/Game/SquidGameBP/Gamemode/BP_SquidInstance` (`GameplayStatics.GetGameInstance`)))
      (switch `int` (`/Game/SquidGameBP/Gamemode/BP_SquidInstance.DiffLevel` _asbp_squid_instance)
        (:`0`
          (set `self.TotalSec` 150.0))
        (:`1`
          (set `self.TotalSec` 60.0))
        (:`2`
          (set `self.TotalSec` 45.0))))
    (:`then_1`
      (bind _asbp_squid_game_mode (cast `/Game/SquidGameBP/Gamemode/BP_SquidGameMode` (`GameplayStatics.GetGameMode`)))
      (add `/Game/SquidGameBP/Gamemode/BP_SquidGameMode.OnLevelStartUp` _asbp_squid_game_mode (delegate `starttime`)))))

(event `starttime`
  (`KismetSystemLibrary.Delay` 4.0)
  (`KismetSystemLibrary.K2_SetTimer` null "UpdateTime" 0.01 true))

(fn `FloatToString`
  (params (Newtime :type "Float (double-precision)"))
  (returns (Result :type String))
  (bind _returnvalue (`KismetMathLibrary.FFloor` Newtime))
  (if (< _returnvalue 10)
    (return (`KismetStringLibrary.Concat_StrStr` "0" (`KismetStringLibrary.Conv_IntToString` _returnvalue)))
    (else
      (return (`KismetStringLibrary.Conv_IntToString` _returnvalue)))))

(fn `UpdateTime`
  ;[1 1 1] 초 단위 누적 처리
  (bind _output_get (set `self.TotalSec` (+ (* (`self.Speed`) 0.01) (`self.TotalSec`))))
  (bind _returnvalue (`KismetMathLibrary.FClamp` _output_get 0.0 300.0))
  (bind _returnvalue_2 (`KismetStringLibrary.Concat_StrStr` (`self.FloatToString` (/ _returnvalue 60.0)) ":" (`self.FloatToString` (mod _returnvalue 60.0))))
  ;[1 1 1] Str 출력 처리
  (if (`KismetStringLibrary.NotEqual_StrStr` _returnvalue_2 (`self.BeforeStr`))
    (bind _output_get_2 (set `self.BeforeStr` _returnvalue_2))
    (`KismetSystemLibrary.PrintString` _output_get_2)
    (`TextRenderComponent.K2_SetText` (`self.TextRender`) (`KismetTextLibrary.Conv_StringToText` _returnvalue_2))
    (if (`KismetStringLibrary.EqualEqual_StrStr` (`self.BeforeStr`) "00:00")
      (`KismetSystemLibrary.PrintString` "타임오버")
      (`self.OnGameTimeOut`)
      (`KismetSystemLibrary.K2_ClearTimer` null "UpdateTime"))))

(fn `UserConstructionScript`)