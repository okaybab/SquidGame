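; Squid Game "Red Light, Green Light" doll that plays the Mugung chant and ragdolls players caught moving.
; Game start triggers the first chant after a delay; the game level feeds the sound's "gamelevel" parameter.
; Audio playback percent drives timing: the Start sound turns the body via timeline, and Mugung's end runs PlayerMoveCheck.
; That check tests velocity of unsafe BP_SquidPersons cached at BeginPlay, then re-arms the chant by timer.
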(event `self.ReceiveBeginPlay`
  (`|ExecutionSequence`
    (:`then_0`
      ;[1 1 1] worker일때는?
      (bind _outactors (`GameplayStatics.GetAllActorsOfClass` "/Game/SquidGameBP/Gamemode/BP_SquidPerson.BP_SquidPerson_C"))
      (bind _output_get (set `self.target` _outactors))
      (for _array_element _output_get
        (`KismetSystemLibrary.PrintString` (`KismetSystemLibrary.GetObjectName` _array_element))))
    (:`then_1`
      (set `self.SoundRandomStop` (`KismetMathLibrary.RandomFloatInRange` 0.1 0.5))
      (set `self.Random Delay` (* (`KismetMathLibrary.Conv_BoolToInt` (`KismetMathLibrary.RandomBool`)) (`KismetMathLibrary.RandomFloatInRange` 4.0 6.0)))
      (bind _asbp_squid_game_mode (cast `/Game/SquidGameBP/Gamemode/BP_SquidGameMode` (`GameplayStatics.GetGameMode`)))
      (bind _difflevel (`/Game/SquidGameBP/Gamemode/BP_SquidGameMode.getGameLevel` _asbp_squid_game_mode))
      (`AudioComponent.SetIntParameter` (`self.mugung`) "gamelevel" _difflevel)
      (add `/Game/SquidGameBP/Gamemode/BP_SquidGameMode.OnGameStart` _asbp_squid_game_mode (delegate `FirstVoice`))
      (`KismetSystemLibrary.PrintString` (`KismetStringLibrary.Conv_IntToString` _difflevel)))))

(event `FirstVoice`
  (`KismetSystemLibrary.Delay` 4.0)
  (`self.onVoice`))

(event `self.ReceiveTick`
  (params (DeltaSeconds :type "Float (single-precision)")))

(event `self.mugung.OnAudioPlaybackPercent`
  (params (PlayingSoundWave :type "SoundWave Object Reference") (PlaybackPercent :type "Float (single-precision)"))
  (if (> PlaybackPercent 0.7)
    (`/Engine/EditorBlueprintResources/StandardMacros.Do N` (`KismetMathLibrary.Conv_BoolToInt` (== PlaybackPercent 1.0)) :!label _label
      (:`Exit`
        (`KismetSystemLibrary.PrintString` "플레이어 체크!")
        (`self.PlayerMoveCheck`)))
    (else
      (goto _label :!via `Reset`))))

(event `self.start.OnAudioPlaybackPercent`
  (params (PlayingSoundWave :type "SoundWave Object Reference") (PlaybackPercent :type "Float (single-precision)"))
  (if (>= PlaybackPercent 0.4)
    (`/Engine/EditorBlueprintResources/StandardMacros.DoOnce` false
      (:`Completed`
        (bind (_direction _bodyrotation) (`Timeline|gamestartbodyrotation`)
          (:`Update`
            (`SceneComponent.K2_SetWorldRotation` (`self.DefaultSceneRoot`) (`KismetMathLibrary.MakeRotator` 0.0 0.0 _bodyrotation) false false)))))))

(fn `onVoice`
  (`ActorComponent.Activate` (`self.mugung`) false))

(fn `PlayerMoveCheck`
  (locals (loop :type Integer))
  (for _array_element (`self.target`)
    (bind _asbp_squid_person (cast `/Game/SquidGameBP/Gamemode/BP_SquidPerson` _array_element))
    (if (`KismetMathLibrary.BooleanNOR` (`/Game/SquidGameBP/Gamemode/BP_SquidPerson.IsSafe` _asbp_squid_person) (not (> (`KismetMathLibrary.VSize` (`self.GetVelocity` _array_element)) 0.0)))
      (`KismetSystemLibrary.PrintString` (`KismetStringLibrary.Concat_StrStr` (`KismetSystemLibrary.GetObjectName` _array_element) " : NOR 죽었다.."))
      (`/Game/SquidGameBP/Gamemode/BP_SquidPerson.DoRacdol` _asbp_squid_person)
      (`KismetSystemLibrary.K2_SetTimer` null "onVoice" 2.0)
      (else
        (`KismetSystemLibrary.PrintString` "살았다!")
        (`KismetSystemLibrary.K2_SetTimer` null "onVoice" 2.0)))))

(fn `SetVolume`
  (params (volume :type "Float (double-precision)"))
  (set `AudioComponent.VolumeMultiplier` volume (`self.mugung`)))

(fn `SoundFlipFlop`)

(fn `UserConstructionScript`)