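; BP_CannonBall is a cannon actor that aims an Arrow at a Target and launches a physics Ball.
; A looping timer eases the Arrow toward the Target using rotator lerp, and a second timer stops tracking after five seconds.
; DoShoot, not called here, resets the Ball to the Arrow, clears its velocity and applies a forward impulse.
; The hit event is empty; ragdoll, knockback and explosion logic for BP_SquidPerson is disconnected.
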(event `self.ReceiveBeginPlay`
  (`KismetSystemLibrary.K2_SetTimer` null "Do Safezone Rotate" 0.1 true)
  (`KismetSystemLibrary.K2_SetTimer` null "DoClearTimer" 5.0))

(event `self.ReceiveTick`
  (params (DeltaSeconds :type "Float (single-precision)")))

(event `self.Ball.OnComponentHit`
  (params (HitComponent :type "PrimitiveComponent Object Reference") (OtherActor :type "Actor Object Reference") (OtherComp :type "PrimitiveComponent Object Reference") (NormalImpulse :type "Vector Structure") (Hit :type "HitResult Structure (by ref)")))

(fn `Do Safezone Rotate`
  (bind _arrow (`self.Arrow`))
  (`SceneComponent.K2_SetWorldRotation` _arrow (`KismetMathLibrary.RLerp` (`SceneComponent.K2_GetComponentRotation` _arrow) (`KismetMathLibrary.FindLookAtRotation` (`SceneComponent.K2_GetComponentLocation` _arrow) (`self.K2_GetActorLocation` (`self.Target`))) 0.05 true) false false))

(fn `Do Shoot`
  (bind _ball (`self.Ball`))
  (bind _arrow (`self.Arrow`))
  (`SceneComponent.K2_SetWorldLocationAndRotation` (`self.Ball`) (`SceneComponent.K2_GetComponentLocation` _arrow) (`SceneComponent.K2_GetComponentRotation` _arrow) false false)
  ;[1 1 1] impulse 물리적인 힘 초기화
  (`PrimitiveComponent.SetAllPhysicsLinearVelocity` _ball (0.0 0.0 0.0) false)
  (`PrimitiveComponent.AddImpulse` _ball (* (`SceneComponent.GetForwardVector` _ball) 5000.0) "None" false))

(fn `DoClearTimer`
  (`KismetSystemLibrary.K2_ClearTimer` null "Do Safezone Rotate"))

(fn `UserConstructionScript`)