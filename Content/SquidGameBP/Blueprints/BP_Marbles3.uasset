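; BP_Marbles3 is a marble pickup that spins, bobs and awards three Ganbu when a BP_SquidPerson overlaps it.
; A fast looping timer, started on BeginPlay, drives MoveActor, which applies a randomized yaw spin and moves the mesh up and down between fixed relative heights.
; On pickup it hides itself, disables mesh collision, plays two sounds and adds to the Ganbu count through BP_SquidGameMode.
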(event `self.ReceiveBeginPlay`
  (`|ExecutionSequence`
    (:`then_0`
      (set `self.Delta Rotation Z (Yaw)` (`KismetMathLibrary.RandomFloatInRange` 0.5 3.0)))
    (:`then_1`
      (`KismetSystemLibrary.K2_SetTimer` null "MoveActor" 0.01 true))))

(event `self.StaticMesh.OnComponentBeginOverlap`
  (params (OverlappedComponent :type "PrimitiveComponent Object Reference") (OtherActor :type "Actor Object Reference") (OtherComp :type "PrimitiveComponent Object Reference") (OtherBodyIndex :type Integer) (bFromSweep :type Boolean) (SweepResult :type "HitResult Structure (by ref)"))
  (cast `/Game/SquidGameBP/Gamemode/BP_SquidPerson` OtherActor)
  (`KismetSystemLibrary.PrintString` "먹었다!")
  (`self.SetActorHiddenInGame` true)
  (`PrimitiveComponent.SetCollisionEnabled` (`self.StaticMesh`) "NoCollision")
  (`AudioComponent.Play` (`self.Audio`) 0.1)
  (`AudioComponent.Play` (`self.Audio1`) 0.0)
  (bind _asbp_squid_game_mode (cast `/Game/SquidGameBP/Gamemode/BP_SquidGameMode` (`GameplayStatics.GetGameMode`)))
  (`/Game/SquidGameBP/Gamemode/BP_SquidGameMode.SetAddGanbu` _asbp_squid_game_mode 3))

(fn `MoveActor`
  (`self.UpdateRotation`)
  (`self.UpdateMoveUpDown` 0.01))

(fn `UpdateMoveUpDown`
  (params (A :type "Float (double-precision)"))
  (bind _staticmesh (`self.StaticMesh`))
  (bind _staticmesh_2 (`self.StaticMesh`))
  (bind _returnvalue (* A (`self.Speed`)))
  (bind (_relativelocation_x _relativelocation_y _relativelocation_z) (`KismetMathLibrary.BreakVector` (`SceneComponent.RelativeLocation` _staticmesh_2)))
  (bind (_relativelocation_x_2 _relativelocation_y_2 _relativelocation_z_2) (`KismetMathLibrary.BreakVector` (`SceneComponent.RelativeLocation` _staticmesh_2)))
  (if (`self.IsRight`)
    (`SceneComponent.K2_AddRelativeLocation` _staticmesh (`KismetMathLibrary.MakeVector` 0.0 0.0 _returnvalue) false false)
    (if (> _relativelocation_z 150.0)
      (set `self.IsRight` false))
    (else
      (bind _result (`/Engine/EditorBlueprintResources/StandardMacros.NegateFloat` _returnvalue)
        (:`  `
          (`SceneComponent.K2_AddRelativeLocation` _staticmesh (`KismetMathLibrary.MakeVector` 0.0 0.0 _result) false false)
          (if (< _relativelocation_z_2 100.0)
            (set `self.IsRight` true)))))))

(fn `UpdateRotation`
  (`SceneComponent.K2_AddRelativeRotation` (`self.StaticMesh`) (`KismetMathLibrary.MakeRotator` 0.0 0.0 (`self.Delta Rotation Z (Yaw)`)) false false))

(fn `UserConstructionScript`)