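; BP_SquidGameMode is the game mode for a Squid Game-style level, coordinating game start and difficulty.
; On BeginPlay it sets game-only input, hides the cursor and binds to the HUD's game-start event.
; On start it activates audio, calls a delayed overlap collision preset change on every BP_Safezone, then broadcasts OnGameStart.
; Getter and setter functions access the difficulty level in BP_SquidInstance, clamped on set.
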(event `self.ReceiveBeginPlay`
  (bind _returnvalue (`GameplayStatics.GetPlayerController` 0))
  (`WidgetBlueprintLibrary.SetInputMode_GameOnly` _returnvalue)
  (set `PlayerController.bShowMouseCursor` false _returnvalue)
  (bind _asbp_squid_hud (cast `/Game/SquidGameBP/Gamemode/BP_SquidHUD` (`PlayerController.GetHUD` (`GameplayStatics.GetPlayerController` 0))))
  (add `/Game/SquidGameBP/Gamemode/BP_SquidHUD.OnGameStart` _asbp_squid_hud (delegate `gamestart`)))

(event `gamestart`
  (`ActorComponent.Activate` (`self.Audio`) false)
  (bind _outactors (`GameplayStatics.GetAllActorsOfClass` "/Game/SquidGameBP/Blueprints/BP_Safezone.BP_Safezone_C"))
  (bind _output_get (set `self.Safezones` _outactors))
  (for _array_element _output_get
    (`/Game/SquidGameBP/Blueprints/BP_Safezone.SetCollisionPreset` _array_element 3.0 "OverlapAllDynamic"))
  (`self.OnGameStart`))

(fn `getGameLevel`
  (returns (DiffLevel :type Integer))
  (bind _asbp_squid_instance (cast `/Game/SquidGameBP/Gamemode/BP_SquidInstance` (`GameplayStatics.GetGameInstance`)))
  (return (`/Game/SquidGameBP/Gamemode/BP_SquidInstance.DiffLevel` _asbp_squid_instance)))

(fn `setGameLevel`
  (params (NewLevel :type Integer))
  (bind _asbp_squid_instance (cast `/Game/SquidGameBP/Gamemode/BP_SquidInstance` (`GameplayStatics.GetGameInstance`)))
  (set `/Game/SquidGameBP/Gamemode/BP_SquidInstance.DiffLevel` (`KismetMathLibrary.Clamp` NewLevel 0 2) _asbp_squid_instance))

(fn `UserConstructionScript`)