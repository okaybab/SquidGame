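; BP_SquidHUD is the HUD for the Squid Game mode, managing the game guide and life widgets.
; On BeginPlay it creates both widgets and shows the life widget at once.
; A six-second timer then displays the guide as a start menu, switching to UI-only input with a visible mouse cursor.
; Functions let other code show or hide the guide and update the life and Ganbu text.
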(event `self.ReceiveBeginPlay`
  (bind _returnvalue (`|CreateWidget` "/Game/SquidGameBP/Widget/gameguideWidget.gameguideWidget_C"))
  (bind _output_get (set `self.guidewidget` _returnvalue))
  (`KismetSystemLibrary.K2_SetTimerDelegate` (delegate `ShowGameStartMenu`) 6.0)
  (bind _returnvalue_2 (`|CreateWidget` "/Game/SquidGameBP/Widget/LifeWidget.LifeWidget_C"))
  (bind _output_get_2 (set `self.lifeWidget` _returnvalue_2))
  (`UserWidget.AddToViewport` _output_get_2 0))

(event `ShowGameStartMenu`
  (bind _returnvalue (`GameplayStatics.GetPlayerController` 0))
  (`UserWidget.AddToViewport` (stale `self.ReceiveBeginPlay` _output_get) 0)
  (`WidgetBlueprintLibrary.SetInputMode_UIOnlyEx` _returnvalue null)
  (set `PlayerController.bShowMouseCursor` true _returnvalue))

(fn `FHideWidget`
  (`/Game/SquidGameBP/Widget/gameguideWidget.HideMenu` (`self.guidewidget`)))

(fn `FShowWidget`
  (bind _guidewidget (`self.guidewidget`))
  (`/Engine/EditorBlueprintResources/StandardMacros.IsValid` _guidewidget
    (:`Is Valid`
      (`/Game/SquidGameBP/Widget/gameguideWidget.ShowMenu` _guidewidget))
    (:`Is Not Valid`
      (`KismetSystemLibrary.PrintString` "위젯 아직 안만들어졌음"))))

(fn `setGanbuText`
  (params (newGanbu :type Text))
  (set `/Game/SquidGameBP/Widget/LifeWidget.txtGanbu` newGanbu (`self.lifeWidget`)))

(fn `setLifeText`
  (params (newLife :type Text))
  (set `/Game/SquidGameBP/Widget/LifeWidget.txtLife` newLife (`self.lifeWidget`)))

(fn `UserConstructionScript`)